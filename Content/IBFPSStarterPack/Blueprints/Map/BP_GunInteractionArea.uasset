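; BP_GunInteractionArea is a pedestal zone where the first-person character can pick up a gun's configuration through shop interaction.
; Box overlap recolors the caption, spawns or destroys a highlight light, toggles shop interaction on the character and registers itself as its active area.
; SetNewVar pushes this area's gun mesh, sights, animations, montages, ID and FX to the stored character.
; Construction creates a dynamic material for the pedestal.
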(event OnComponentEndOverlap(Box)
  (params (OverlappedComponent :type Primitive%20Component%20Object%20Reference) (OtherActor :type Actor%20Object%20Reference) (OtherComp :type Primitive%20Component%20Object%20Reference) (OtherBodyIndex :type Integer))
  ;[1 1 1] Disable interaction when overaly end
  ;;[1 1 1] Set label color to default
  (Rendering|Components|TextRender|SetTextRenderColor (Variables|/Script/Engine.TextRenderActor|GetTextRender (Variables|Default|GetCaption)) (Math|Conversions|ToColor(LinearColor) (Variables|Default|GetDefaultColor)))
  (Variables|Default|SetInteractionEnabled false)
  (bind _asfirst_person_character_fpsstarter_kit_v2 (Utilities|Casting|CastToFirstPersonCharacter_FPSStarterKitV2 OtherActor))
  ;;[1 1 1] Remove light point
  (Actor|DestroyActor (Variables|Default|GetLightSpawned))
  (Variables|/Game/IBFPSStarterPack/Blueprints/FirstPersonCharacter_FPSStarterKitV2.FirstPersonCharacter_FPSStarterKitV2_C|SetbEnableShopInteraction _asfirst_person_character_fpsstarter_kit_v2 false))

(event OnComponentBeginOverlap(Box)
  (params (OverlappedComponent :type Primitive%20Component%20Object%20Reference) (OtherActor :type Actor%20Object%20Reference) (OtherComp :type Primitive%20Component%20Object%20Reference) (OtherBodyIndex :type Integer) (bFromSweep :type Boolean) (SweepResult :type Hit%20Result%20Structure%20%28by%20ref%29))
  ;[1 1 1] Enable interaction when overaly begin
  (Variables|Default|SetInteractionEnabled true)
  (bind _asfirst_person_character_fpsstarter_kit_v2 (Utilities|Casting|CastToFirstPersonCharacter_FPSStarterKitV2 (Game|GetPlayerCharacter 0)))
  ;;[1 1 1] Set label color
  (Rendering|Components|TextRender|SetTextRenderColor (Variables|/Script/Engine.TextRenderActor|GetTextRender (Variables|Default|GetCaption)) (Math|Conversions|ToColor(LinearColor) (Variables|Default|GetEnabledColor)))
  ;;[1 1 1] Spawn LightPoint actor
  (bind _returnvalue (Game|SpawnActorfromClass "/Game/IBFPSStarterPack/Blueprints/Map/BP_LightActor.BP_LightActor_C" (Transformation|GetWorldTransform (Variables|Default|GetLightPosition)) "Undefined" 0 0))
  (Variables|Default|SetLightSpawned _returnvalue)
  (Variables|/Game/IBFPSStarterPack/Blueprints/FirstPersonCharacter_FPSStarterKitV2.FirstPersonCharacter_FPSStarterKitV2_C|SetInteractionArea _asfirst_person_character_fpsstarter_kit_v2 self)
  (Variables|/Game/IBFPSStarterPack/Blueprints/FirstPersonCharacter_FPSStarterKitV2.FirstPersonCharacter_FPSStarterKitV2_C|SetbEnableShopInteraction _asfirst_person_character_fpsstarter_kit_v2 true)
  (Variables|Default|SetCharacter_reference _asfirst_person_character_fpsstarter_kit_v2))

(event Custom|SetNewVar
  ;[1 1 1] Set gun vars to mainCharacter
  (Default|SetNewGunStuff (Variables|Default|GetCharacter_reference) (Variables|Default|GetGunSkeletalMesh) (Variables|Default|GetIronSight) (Variables|Default|GetGun_FireMontage) (Variables|Default|GetGun_IdleAnim) (Variables|Default|GetGun_ReloadMontage) (Variables|Default|GetGun_AnimBlueprint) (Variables|Default|GetGun_ADSFireMontage) (Variables|Default|GetArms_FireMontage) (Variables|Default|GetArms_ADSFireMontage) (Variables|Default|GetArms_ReloadMontage) (Variables|Default|GetArms_RaiseMontage) (Variables|Default|GetArms_LowerMontage) (Variables|Default|GetGunId) (Variables|Default|GetFX)))

(fn ConstructionScript
  (bind _returnvalue (Rendering|Material|CreateDynamicMaterialInstance (Variables|/Script/Engine.StaticMeshActor|GetStaticMeshComponent (Variables|Default|GetPedestal)) 0 0 :!class /Script/Engine.PrimitiveComponent))
  (LocalVariables|SetPedestalMaterialInstance _returnvalue))

(fn TestActive
  (return (Variables|Default|GetInteractionEnabled)))