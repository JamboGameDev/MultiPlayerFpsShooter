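; Map display area that showcases animated first-person arms and lets the FPS starter kit player interact with it as a shop.
; Entering the box highlights the caption, spawns a light, loops random unarmed animations on twelve arms actors and registers the area on the player character.
; Leaving it reverses these changes.
; GetArms returns a randomly picked arms variant, while the pedestal emissive and direct arms-swap nodes are left unconnected.
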(event `AnimateAll`
  (bind _output_get (set `self.ArmsAnimatedArray` (`|MakeArray` (`self.ArmsAnimated`) (`self.ArmsAnimated_0`) (`self.ArmsAnimated_1`) (`self.ArmsAnimated_2`) (`self.ArmsAnimated_3`) (`self.ArmsAnimated_4`) (`self.ArmsAnimated_5`) (`self.ArmsAnimated_7`) (`self.ArmsAnimated_8`) (`self.ArmsAnimated_9`) (`self.ArmsAnimated_10`) (`self.ArmsAnimated_6`))))
  (for _array_element _output_get
    (switch `int` (`KismetMathLibrary.RandomInteger` 5)
      (:`0`
        (bind _skeletalmeshcomponent (`SkeletalMeshActor.SkeletalMeshComponent` _array_element))
        (`SkeletalMeshComponent.PlayAnimation` _skeletalmeshcomponent "/Game/FpsShooter/AnimationsHand/Arms/ANIM_Unarmed_Idle.ANIM_Unarmed_Idle" true))
      (:`1`
        (`SkeletalMeshComponent.PlayAnimation` _skeletalmeshcomponent "/Game/FpsShooter/AnimationsHand/Arms/ANIM_Unarmed_Jump.ANIM_Unarmed_Jump" true))
      (:`2`
        (`SkeletalMeshComponent.PlayAnimation` _skeletalmeshcomponent "/Game/FpsShooter/AnimationsHand/Arms/ANIM_Unarmed_Punch.ANIM_Unarmed_Punch" true))
      (:`3`
        (`SkeletalMeshComponent.PlayAnimation` _skeletalmeshcomponent "/Game/FpsShooter/AnimationsHand/Arms/ANIM_Unarmed_Push_Door.ANIM_Unarmed_Push_Door" true))
      (:`4`
        (`SkeletalMeshComponent.PlayAnimation` _skeletalmeshcomponent "/Game/FpsShooter/AnimationsHand/Arms/ANIM_Unarmed_Sprint.ANIM_Unarmed_Sprint" true)))
    (`SkeletalMeshComponent.SetPlayRate` _skeletalmeshcomponent 0.75)))

(event `SetNewVar`
  (bind _activestatus (`self.TestActive`))
  (if _activestatus
    _))

(event `EndAnimations`
  (for _array_element (`self.ArmsAnimatedArray`)
    (`SkeletalMeshComponent.Stop` (`SkeletalMeshActor.SkeletalMeshComponent` _array_element))))

(event `self.Box.OnComponentBeginOverlap`
  (params (OverlappedComponent :type "PrimitiveComponent Object Reference") (OtherActor :type "Actor Object Reference") (OtherComp :type "PrimitiveComponent Object Reference") (OtherBodyIndex :type Integer) (bFromSweep :type Boolean) (SweepResult :type "HitResult Structure (by ref)"))
  (set `self.InteractionEnabled` true)
  (bind _asfirst_person_character_fpsstarter_kit_v2 (cast `/Game/IBFPSStarterPack/Blueprints/FirstPersonCharacter_FPSStarterKitV2` (`GameplayStatics.GetPlayerCharacter` 0)))
  (`TextRenderComponent.SetTextRenderColor` (`TextRenderActor.TextRender` (`self.Caption`)) (`KismetMathLibrary.Conv_LinearColorToColor` (`self.EnabledColor`)))
  (bind _returnvalue (`|SpawnActorFromClass` "/Game/IBFPSStarterPack/Blueprints/Map/BP_LightActor.BP_LightActor_C" (`SceneComponent.K2_GetComponentToWorld` (`self.LightPosition`)) "Undefined" "OverrideRootScale" null null))
  (set `self.LightSpawned` _returnvalue)
  (`self.AnimateAll`)
  (set `/Game/IBFPSStarterPack/Blueprints/FirstPersonCharacter_FPSStarterKitV2.InteractionArea` self _asfirst_person_character_fpsstarter_kit_v2)
  (set `/Game/IBFPSStarterPack/Blueprints/FirstPersonCharacter_FPSStarterKitV2.bEnableShopInteraction` true _asfirst_person_character_fpsstarter_kit_v2))

(event `self.Box.OnComponentEndOverlap`
  (params (OverlappedComponent :type "PrimitiveComponent Object Reference") (OtherActor :type "Actor Object Reference") (OtherComp :type "PrimitiveComponent Object Reference") (OtherBodyIndex :type Integer))
  (set `self.InteractionEnabled` false)
  (bind _asfirst_person_character_fpsstarter_kit_v2 (cast `/Game/IBFPSStarterPack/Blueprints/FirstPersonCharacter_FPSStarterKitV2` OtherActor))
  (`self.EndAnimations`)
  (`TextRenderComponent.SetTextRenderColor` (`TextRenderActor.TextRender` (`self.Caption`)) (`KismetMathLibrary.Conv_LinearColorToColor` (`self.DefaultColor`)))
  (`self.K2_DestroyActor` (`self.LightSpawned`))
  (set `/Game/IBFPSStarterPack/Blueprints/FirstPersonCharacter_FPSStarterKitV2.bEnableShopInteraction` false _asfirst_person_character_fpsstarter_kit_v2)
  (set `/Game/IBFPSStarterPack/Blueprints/FirstPersonCharacter_FPSStarterKitV2.InteractionArea` null _asfirst_person_character_fpsstarter_kit_v2))

(fn `GetArms`
  (returns (Arms :type "SkeletalMesh Object Reference"))
  (locals (SelectedArms :type "SkeletalMesh Object Reference"))
  ;[1 1 1] Change arms randomly
  (switch `int` (`KismetMathLibrary.RandomInteger` 11)
    (:`Default`
      _)
    (:`0`
      (bind _output_get (set `local.SelectedArms` (`self.Arms`)))
      (return _output_get))
    (:`1`
      (bind _output_get_2 (set `local.SelectedArms` (`self.Arms_0`)))
      (return _output_get_2))
    (:`2`
      (bind _output_get_3 (set `local.SelectedArms` (`self.Arms_2`)))
      (return _output_get_3))
    (:`3`
      (bind _output_get_4 (set `local.SelectedArms` (`self.Arms_3`)))
      (return _output_get_4))
    (:`4`
      (bind _output_get_5 (set `local.SelectedArms` (`self.Arms_4`)))
      (return _output_get_5))
    (:`5`
      (bind _output_get_6 (set `local.SelectedArms` (`self.Arms_5`)))
      (return _output_get_6))
    (:`6`
      (bind _output_get_7 (set `local.SelectedArms` (`self.Arms_6`)))
      (return _output_get_7))
    (:`7`
      (bind _output_get_8 (set `local.SelectedArms` (`self.Arms_7`)))
      (return _output_get_8))
    (:`8`
      (bind _output_get_9 (set `local.SelectedArms` (`self.Arms_8`)))
      (return _output_get_9))
    (:`9`
      (bind _output_get_10 (set `local.SelectedArms` (`self.Arms_9`)))
      (return _output_get_10))
    (:`10`
      (bind _output_get_11 (set `local.SelectedArms` (`self.Arms_10`)))
      (return _output_get_11))
    (:`11`
      _))
  (bind _output_get_12 (set `local.SelectedArms` (`self.Arms_11`)))
  (return _output_get_12))

(fn `TestActive`
  (returns (ActiveStatus :type Boolean))
  (return (`self.InteractionEnabled`)))

(fn `UserConstructionScript`
  (locals (PedestalMaterialInstance :type "MaterialInstanceDynamic Object Reference"))
  (bind _returnvalue (`PrimitiveComponent.CreateDynamicMaterialInstance` (`StaticMeshActor.StaticMeshComponent` (`self.Pedestal`)) 0 null "None"))
  (set `local.PedestalMaterialInstance` _returnvalue))