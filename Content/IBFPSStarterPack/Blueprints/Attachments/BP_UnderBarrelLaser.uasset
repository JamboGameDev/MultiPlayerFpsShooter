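; Under-barrel laser attachment for the first-person character that aims a beam mesh and an impact light each tick.
; The trace origin switches between the laser source (reloading or sprinting), first-person camera, or scope camera for an M233 sight.
; A visibility trace from that origin positions the light and rotates and stretches the beam, skipping updates on Ironbelly projectile hits.
; The beam hides while aiming through an attached sight.
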(event `self.ReceiveBeginPlay`)

(event `self.ReceiveTick`
  (params (DeltaSeconds :type "Float (single-precision)"))
  (bind _laserimpactlight (`self.LaserImpactLight`))
  (bind _sm_laserbeam (`self.SM_LaserBeam`))
  (bind _aimingcomponent (`self.AimingComponent`))
  (bind _returnvalue (`SceneComponent.K2_GetComponentLocation` _aimingcomponent))
  (bind _returnvalue_2 (+ _returnvalue (* (`SceneComponent.GetForwardVector` _aimingcomponent) 10000.0)))
  (bind _asfirst_person_character_fpsstarter_kit_v2 (cast `/Game/IBFPSStarterPack/Blueprints/FirstPersonCharacter_FPSStarterKitV2` (`GameplayStatics.GetPlayerCharacter` 0)))
  (if (or (`/Game/IBFPSStarterPack/Blueprints/FirstPersonCharacter_FPSStarterKitV2.bReloading` _asfirst_person_character_fpsstarter_kit_v2) (`/Game/IBFPSStarterPack/Blueprints/FirstPersonCharacter_FPSStarterKitV2.bSprinting` _asfirst_person_character_fpsstarter_kit_v2))
    (set `self.AimingComponent` (`self.LaserSource`))
    (elif (`/Game/IBFPSStarterPack/Blueprints/FirstPersonCharacter_FPSStarterKitV2.bAiming` _asfirst_person_character_fpsstarter_kit_v2)
      (bind _attachedsight (`/Game/IBFPSStarterPack/Blueprints/FirstPersonCharacter_FPSStarterKitV2.AttachedSight` _asfirst_person_character_fpsstarter_kit_v2))
      (`/Engine/EditorBlueprintResources/StandardMacros.IsValid` _attachedsight
        (:`Is Valid`
          ;[1 1 1] Check if big scope attached
          (castclass `/Game/IBFPSStarterPack/Blueprints/Attachments/BP_M233` (`GameplayStatics.GetObjectClass` _attachedsight)
            (:`then`
              (set `self.AimingComponent` (`/Game/IBFPSStarterPack/Blueprints/FirstPersonCharacter_FPSStarterKitV2.ScopeCamera` _asfirst_person_character_fpsstarter_kit_v2)))
            (:`CastFailed`
              (bind _firstpersoncamera (`/Game/IBFPSStarterPack/Blueprints/FirstPersonCharacter_FPSStarterKitV2.FirstPersonCamera` _asfirst_person_character_fpsstarter_kit_v2))
              (set `self.AimingComponent` _firstpersoncamera)))
          (`SceneComponent.SetVisibility` (`self.SM_LaserBeam`) false false))
        (:`Is Not Valid`
          (set `self.AimingComponent` _firstpersoncamera :!label _label)
          (`SceneComponent.SetVisibility` (`self.SM_LaserBeam`) true false)))
      (else
        (goto _label))))
  (bind (_outhit _returnvalue_3) (`KismetSystemLibrary.LineTraceSingle` _returnvalue _returnvalue_2 "TraceTypeQuery1"))
  (bind (_bblockinghit _binitialoverlap _time _location _impactpoint _normal _impactnormal _physmat _hitactor) (`GameplayStatics.BreakHitResult` _outhit))
  (cast `/Game/IBFPSStarterPack/Blueprints/BP_FirstPersonProjectileIronbelly` _hitactor
    (:`CastFailed`
      (cast `/Game/IBFPSStarterPack/Blueprints/BP_FirstPersonProjectileIronbellyFast` _hitactor
        (:`CastFailed`
          (if _returnvalue_3
            (set `self.LaserTargetLocation` _location)
            (else
              (set `self.LaserTargetLocation` _returnvalue_2)))
          (`SceneComponent.K2_SetWorldLocation` _laserimpactlight (- (`self.LaserTargetLocation`) (`SceneComponent.GetForwardVector` _laserimpactlight)) false false)
          (`SceneComponent.SetWorldScale3D` _sm_laserbeam (`KismetMathLibrary.MakeVector` (`KismetMathLibrary.VSize` (- _returnvalue _impactpoint)) 1.0 1.0))
          (`SceneComponent.K2_SetWorldRotation` _sm_laserbeam (`KismetMathLibrary.FindLookAtRotation` (`SceneComponent.K2_GetComponentLocation` (`self.LaserSource`)) (`self.LaserTargetLocation`)) false false))))))

(fn `UserConstructionScript`
  (`parent.UserConstructionScript`))